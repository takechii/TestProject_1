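; BP_GrabBaseV2 is a base actor, named for grabbing, with a balance meter that damage drains until it breaks.
; Construction fills the balance to its maximum; AnyDamage lowers it, updates the gauge widget's progress and sets BalanceBreak at zero.
; BeginPlay caches the gauge and direction widgets from its widget components, hides the direction indicator and stores a reference to the player pawn.
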(event EventBeginPlay
  (Utilities|FlowControl|Sequence
    (:then_0
      (bind _aswbp_sample_gage_v1 (Utilities|Casting|CastToWBP_SampleGageV1 (UserInterface|GetUserWidgetObject (Variables|Default|GetWidget))))
      (Variables|Default|SetAs%20WBP%20SampleGage1 _aswbp_sample_gage_v1)
      (bind _aswbp_sample_direction_v1 (Utilities|Casting|CastToWBP_SampleDirectionV1 (UserInterface|GetUserWidgetObject (Variables|Default|GetWidget1))))
      (bind _output_get (Variables|Default|SetAs%20WBP%20Sample%20Direction%20V1 _aswbp_sample_direction_v1))
      (Default|IsNotShow _output_get))
    (:then_1
      (bind _asbp_player_base_v2 (Utilities|Casting|CastToBP_PlayerBaseV2 (Game|Player|GetPlayerPawn 0)))
      (Variables|Default|SetAs%20BP%20Player%20Base%20V2 _asbp_player_base_v2))))

(event Collision|EventActorBeginOverlap
  (params (OtherActor :type Actor%20Object%20Reference)))

(event EventTick
  (params (DeltaSeconds :type Float%20%28single-precision%29)))

(event Game|Damage|EventAnyDamage
  (params (Damage :type Float%20%28single-precision%29) (DamageType :type Damage%20Type%20Object%20Reference) (InstigatedBy :type Controller%20Object%20Reference) (DamageCauser :type Actor%20Object%20Reference))
  (bind _output_get (Variables|Default|SetCurrent%20Balance%20Point (Math|Float|Max(Float) (- (Variables|Default|GetCurrent%20Balance%20Point) Damage) 0.0)))
  (if (Math|Float|NearlyEqual(Float) _output_get 0.0 1e-06)
    (Default|UpdateHealthProgress (Variables|Default|GetAs%20WBP%20SampleGage1) 0.0)
    (Variables|Default|SetBalance%20Break true)
    (else
      (Default|UpdateHealthProgress (Variables|Default|GetAs%20WBP%20SampleGage1) (/ (Variables|Default|GetCurrent%20Balance%20Point) (Variables|Default|GetMax%20Balance%20Point))))))

(fn ConstructionScript
  (Variables|Default|SetCurrent%20Balance%20Point (Variables|Default|GetMax%20Balance%20Point)))