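; Player character base that moves, jumps, locks on to BP_GrabBaseV2 actors and grabs them.
; A state enum drives input and Tick: lock-on faces the mesh at the target, cycles on press and releases on hold.
; Grabbing enters Battle when in range; from lock-on, distant targets start a lerp timeline toward them.
; Battle ticks damage and recovery of a grasp-point pool shown on a widget gauge, flagging a break at zero.
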(event Custom|Recovery%20Slow%20Gage
  (if (Variables|Default|GetRecovery)
    (if (< (Variables|Default|GetCurrent%20Grasped%20Point) (Variables|Default|GetRecovery%20Value))
      (Variables|Default|SetCurrent%20Grasped%20Point (Math|Float|Min(Float) (+ (Variables|Default|GetCurrent%20Grasped%20Point) 3.0) (Variables|Default|GetMax%20Grasped%20Point)))
      (Default|UpdateHealthProgress (Variables|Default|GetSampleGage1) (/ (Variables|Default|GetCurrent%20Grasped%20Point) (Variables|Default|GetMax%20Grasped%20Point)))
      (Variables|Default|SetBreak false)
      (else
        (Variables|Default|SetRecovery%20Value -5e+02)
        (Variables|Default|SetRecovery false)))))

(event Custom|Damage%20Slow%20Gage
  (if (Variables|Default|GetDamage)
    (bind _output_get (Variables|Default|SetCurrent%20Grasped%20Point (Math|Float|Max(Float) (- (Variables|Default|GetCurrent%20Grasped%20Point) (Variables|Default|GetDamage%20Value)) 0.0)))
    (if (Math|Float|NearlyEqual(Float) _output_get 0.0 1e-06)
      (Default|UpdateHealthProgress (Variables|Default|GetSampleGage1) 0.0)
      (Variables|Default|SetBreak true)
      (else
        (Default|UpdateHealthProgress (Variables|Default|GetSampleGage1) (/ (Variables|Default|GetCurrent%20Grasped%20Point) (Variables|Default|GetMax%20Grasped%20Point)))
        (Variables|Default|SetBreak false)))))

(event Custom|Event%20Recovery
  (params (Recovery%20Value :type Float%20%28double-precision%29))
  (Variables|Default|SetRecovery%20Value (Math|Float|Min(Float) (+ (Variables|Default|GetCurrent%20Grasped%20Point) Recovery%20Value) (Variables|Default|GetMax%20Grasped%20Point)))
  (Variables|Default|SetRecovery true))

(event Custom|Event%20Damage
  (Variables|Default|SetDamage true))

(event Input|EnhancedActionEvents|EnhancedInputActionIA_Jump
  (params (ActionValue :type Boolean) (ElapsedSeconds :type Float%20%28double-precision%29) (TriggeredSeconds :type Float%20%28double-precision%29) (InputAction :type Input%20Action%20Object%20Reference :default "/Game/DefaultSetting/inputAction/IA_Jump.IA_Jump"))
  ;[0 0.3501 1] Input Action -Jumping-
  (:Triggered
    (Character|Jump))
  (:Completed
    (Character|StopJumping)))

(event Input|EnhancedActionEvents|EnhancedInputActionIA_Move
  (params (ActionValue :type Vector%202D%20Structure) (ElapsedSeconds :type Float%20%28double-precision%29) (TriggeredSeconds :type Float%20%28double-precision%29) (InputAction :type Input%20Action%20Object%20Reference :default "/Game/DefaultSetting/inputAction/IA_Move.IA_Move"))
  (bind _returnvalue (Pawn|GetControlRotation :!class /Script/Engine.Pawn))
  ;[0 0.7859 1] Input Action -Moving-
  (:Triggered
    ;;[1 1 1] Always Updated When Inputting
    (Utilities|Array|SetArrayElem (Variables|Default|GetController%20Action%20Value) 0 (.x ActionValue))
    (Utilities|Array|SetArrayElem (Variables|Default|GetController%20Action%20Value) 1 (.y ActionValue))
    (switch Utilities|FlowControl|Switch|SwitchonPBaseV2State (Variables|Default|GetCurrent%20State)
      (:NewEnumerator0
        _)
      (:NewEnumerator1
        _))
    (Pawn|Input|AddMovementInput (Math|Vector|GetRightVector (Math|Rotator|MakeRotator (.roll _returnvalue) 0.0 (.yaw _returnvalue))) (Utilities|Array|Get(acopy) (Variables|Default|GetController%20Action%20Value)) false)
    (Pawn|Input|AddMovementInput (Math|Vector|GetForwardVector (Math|Rotator|MakeRotator 0.0 0.0 (.yaw (Pawn|GetControlRotation :!class /Script/Engine.Pawn)))) (Utilities|Array|Get(acopy) (Variables|Default|GetController%20Action%20Value) 1) false)
    (bind _degree (CallFunction|GetAnglefromZero (Utilities|Array|Get(acopy) (Variables|Default|GetController%20Action%20Value) 1) (Utilities|Array|Get(acopy) (Variables|Default|GetController%20Action%20Value))))
    (Transformation|SetWorldRotation (Variables|Character|GetMesh) (Math|Rotator|MakeRotator 0.0 0.0 (+ _degree -9e+01)) false false))
  (:Started
    ;;[1 1 1] First Of Inputting
    (Utilities|Array|SetArrayElem (Variables|Default|GetController%20Action%20Value) 2 (.x ActionValue))
    (Utilities|Array|SetArrayElem (Variables|Default|GetController%20Action%20Value) 3 (.y ActionValue)))
  (:Completed
    ;;[1 1 1] Reset Array
    (for (_ _array_index) (Variables|Default|GetController%20Action%20Value)
      (Utilities|Array|SetArrayElem (Variables|Default|GetController%20Action%20Value) _array_index 0.0))
    (Development|PrintString "Action Value Resetting!" true true "(R=0.045263,G=1.000000,B=0.000000,A=1.000000)")))

(event Input|EnhancedActionEvents|EnhancedInputActionIA_LockOn
  (params (ActionValue :type Boolean) (ElapsedSeconds :type Float%20%28double-precision%29) (TriggeredSeconds :type Float%20%28double-precision%29) (InputAction :type Input%20Action%20Object%20Reference :default "/Game/DefaultSetting/inputAction/IA_LockOn.IA_LockOn"))
  ;[0 1 0.6898] Input Action -LockOn-
  (:Triggered
    (Utilities|IsValid (Utilities|Array|Get(acopy) (Variables|Default|GetGrasped%20Actors))
      (:Is%20Valid
        (switch Utilities|FlowControl|Switch|SwitchonPBaseV2State (Variables|Default|GetCurrent%20State)
          (:NewEnumerator1
            (bind _result (Math|Integer|IncrementInt (Variables|Default|GetVariables%20Count%20For%20Lock%20On%20Release))
              (:%20%20
                (if (> (Math|Conversions|ToFloat(Integer) _result) (/ 1.0 (Utilities|Time|GetWorldDeltaSeconds)))
                  (Variables|Default|SetVariables%20Count%20For%20Lock%20On%20Release 0)
                  (Variables|Default|SetCurrent%20State "NewEnumerator0")))))))))
  (:Started
    (Utilities|IsValid (Utilities|Array|Get(acopy) (Variables|Default|GetGrasped%20Actors))
      (:Is%20Valid
        (switch Utilities|FlowControl|Switch|SwitchonPBaseV2State (Variables|Default|GetCurrent%20State)
          (:NewEnumerator0
            (for (_array_element _array_index) (Variables|Default|GetGrasped%20Actors)
              (if (> (Variables|Default|GetVariables%20For%20Lock%20On%20Distance) (Math|Vector|Distance(Vector) (Transformation|GetActorLocation _array_element) (Transformation|GetActorLocation)))
                (Variables|Default|SetVariables%20For%20Lock%20On%20Distance (Math|Vector|Distance(Vector) (Transformation|GetActorLocation _array_element) (Transformation|GetActorLocation)))
                (Variables|Default|SetCurrent%20Grasped%20Actor%20Index _array_index)))
            (Variables|Default|SetCurrent%20State "NewEnumerator1")
            (Transformation|SetActorRotation (Math|Rotator|FindLookatRotation (Transformation|GetActorLocation) (Transformation|GetActorLocation (Utilities|Array|Get(acopy) (Variables|Default|GetGrasped%20Actors) (Variables|Default|GetCurrent%20Grasped%20Actor%20Index))))))
          (:NewEnumerator1
            (Math|Integer|IncrementInt (Variables|Default|GetCurrent%20Grasped%20Actor%20Index)
              (:%20%20
                (if (> (Variables|Default|GetCurrent%20Grasped%20Actor%20Index) (- (Utilities|Array|Length (Variables|Default|GetGrasped%20Actors)) 1))
                  (Variables|Default|SetCurrent%20Grasped%20Actor%20Index 0)))))))))
  (:Completed
    (Variables|Default|SetVariables%20Count%20For%20Lock%20On%20Release 0)))

(event Input|EnhancedActionEvents|EnhancedInputActionIA_Grab
  (params (ActionValue :type Boolean) (ElapsedSeconds :type Float%20%28double-precision%29) (TriggeredSeconds :type Float%20%28double-precision%29) (InputAction :type Input%20Action%20Object%20Reference :default "/Game/DefaultSetting/inputAction/IA_Grab.IA_Grab"))
  ;[0.0612 1 0] Input Action -Grab-
  (:Started
    (Utilities|IsValid (Utilities|Array|Get(acopy) (Variables|Default|GetGrasped%20Actors))
      (:Is%20Valid
        (switch Utilities|FlowControl|Switch|SwitchonPBaseV2State (Variables|Default|GetCurrent%20State)
          (:NewEnumerator0
            (if (< (Math|Vector|Distance(Vector) (Transformation|GetActorLocation) (Transformation|GetActorLocation (Utilities|Array|Get(acopy) (Variables|Default|GetGrasped%20Actors) (Variables|Default|GetCurrent%20Grasped%20Actor%20Index)))) (Variables|Default|GetGrasping%20Distance))
              (Variables|Default|SetCurrent%20State "NewEnumerator3")
              (Variables|Default|SetLock%20On%20First%20Location (Transformation|GetActorLocation))
              (bind _output_get (Variables|Default|SetGrasped%20Actor (Utilities|Array|Get(acopy) (Variables|Default|GetGrasped%20Actors) (Variables|Default|GetCurrent%20Grasped%20Actor%20Index))))
              (Variables|/Game/member/Okajima/bp/BP_GrabBaseV2.BP_GrabBaseV2_C|SetCurrent%20State _output_get "NewEnumerator1")
              (CallFunction|EventDamage)))
          (:NewEnumerator1
            (if (> (Math|Vector|Distance(Vector) (Transformation|GetActorLocation) (Transformation|GetActorLocation (Utilities|Array|Get(acopy) (Variables|Default|GetGrasped%20Actors) (Variables|Default|GetCurrent%20Grasped%20Actor%20Index)))) (Variables|Default|GetGrasping%20Distance))
              (Variables|Default|SetCurrent%20State "NewEnumerator2")
              (Variables|Default|SetLock%20On%20First%20Location (Transformation|GetActorLocation))
              (Variables|Default|SetGrasped%20Actor (Utilities|Array|Get(acopy) (Variables|Default|GetGrasped%20Actors) (Variables|Default|GetCurrent%20Grasped%20Actor%20Index)))
              (Components|Timeline|PlayfromStart (Variables|Default|GetLock%20On%20Moving))
              (else
                (Variables|Default|SetCurrent%20State "NewEnumerator3")
                (Variables|Default|SetLock%20On%20First%20Location (Transformation|GetActorLocation))
                (bind _output_get_2 (Variables|Default|SetGrasped%20Actor (Utilities|Array|Get(acopy) (Variables|Default|GetGrasped%20Actors) (Variables|Default|GetCurrent%20Grasped%20Actor%20Index))))
                (Variables|/Game/member/Okajima/bp/BP_GrabBaseV2.BP_GrabBaseV2_C|SetCurrent%20State _output_get_2 "NewEnumerator1")
                (CallFunction|EventDamage)))))))))

(event EventBeginPlay
  (Utilities|FlowControl|Sequence
    (:then_0
      ;[1 1 1] Input Action Bind
      (bind _asplayer_controller (Utilities|Casting|CastToPlayerController (Pawn|GetController)))
      (Utilities|IsValid (PlayerController|LocalPlayerSubsystems|GetEnhancedInputLocalPlayerSubsystem _asplayer_controller)
        (:Is%20Valid
          (Input|AddMappingContext (PlayerController|LocalPlayerSubsystems|GetEnhancedInputLocalPlayerSubsystem _asplayer_controller) "/Game/DefaultSetting/IMC_Default.IMC_Default" 0 "(bIgnoreAllPressedKeysUntilRelease=True,bForceImmediately=False)"))))
    (:then_1
      ;[1 1 1] Setting Grab Actor
      (bind _outactors (Actor|GetAllActorsOfClass "/Game/member/Okajima/bp/BP_GrabBaseV2.BP_GrabBaseV2_C"))
      (Variables|Default|SetGrasped%20Actors _outactors)
      (Variables|Default|SetGrasped%20Actor 0))
    (:then_2
      ;[1 1 1] Setting Default Current State
      (Variables|Default|SetCurrent%20State "NewEnumerator0"))
    (:then_3
      ;[1 1 1] Setting Slow Gage
      (bind _aswbp_sample_gage_v1 (Utilities|Casting|CastToWBP_SampleGageV1 (UserInterface|GetUserWidgetObject (Variables|Default|GetWidget))))
      (bind _output_get (Variables|Default|SetSampleGage1 _aswbp_sample_gage_v1))
      (Default|UpdateHealthProgress _output_get (/ (Variables|Default|GetCurrent%20Grasped%20Point) (Variables|Default|GetMax%20Grasped%20Point))))))

(event Collision|EventActorBeginOverlap
  (params (OtherActor :type Actor%20Object%20Reference)))

(event EventTick
  (params (DeltaSeconds :type Float%20%28single-precision%29))
  (Utilities|FlowControl|Sequence
    (:then_0
      (switch Utilities|FlowControl|Switch|SwitchonPBaseV2State (Variables|Default|GetCurrent%20State)
        (:NewEnumerator1
          (CallFunction|Lockon))
        (:NewEnumerator3
          (CallFunction|Battle))))))

(fn ConstructionScript
  (Variables|Default|SetCurrent%20Grasped%20Point (- (Variables|Default|GetMax%20Grasped%20Point) 5e+01)))

(fn GetAnglefromZero
  (params (X :type Float%20%28double-precision%29) (Y :type Float%20%28double-precision%29))
  (return (/ (* (Math|Trig|Atan2(Radians) (- Y 0.0) (- X 0.0)) 1.8e+02) 3.14)))

(fn Lockon
  (bind _returnvalue (Transformation|GetActorLocation))
  (bind _grasped_actors (Variables|Default|GetGrasped%20Actors))
  (bind _current_grasped_actor_index (Variables|Default|GetCurrent%20Grasped%20Actor%20Index))
  (bind _output (Utilities|Array|Get(acopy) _grasped_actors _current_grasped_actor_index))
  (bind _returnvalue_2 (Transformation|GetActorLocation _output))
  (bind _returnvalue_3 (Math|Rotator|FindLookatRotation _returnvalue _returnvalue_2))
  (bind (_roll _pitch _yaw) (Math|Rotator|BreakRotator _returnvalue_3))
  (Transformation|SetWorldRotation (Variables|Character|GetMesh) (Math|Rotator|MakeRotator _roll _pitch (+ _yaw -9e+01)) false false))

(fn Battle
  (Utilities|FlowControl|Sequence
    (:then_0
      (CallFunction|RecoverySlowGage))
    (:then_1
      (CallFunction|DamageSlowGage))))