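; BP_GrabActorT1V2 is a grab actor that faces the player and picks a random pulling direction during its Battle state.
; Tick runs Battle, which turns the mesh toward the player each frame with a -90 yaw offset.
; Once, while Attack is false, it rolls two PullingDirection axes, randomly adjusts zero or diagonal results, and saves its location.
; Nothing here applies the pull: the movement input is unconnected and Attack is never reset.
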(event EventBeginPlay
  (|CallParentFunction) ; このノードは無効になっているため呼び出せません。\n機能をビルドするにはピンをドラッグしてください。
)

(event Collision|EventActorBeginOverlap
  (params (OtherActor :type Actor%20Object%20Reference))
  (|CallParentFunction OtherActor) ; このノードは無効になっているため呼び出せません。\n機能をビルドするにはピンをドラッグしてください。
)

(event EventTick
  (params (DeltaSeconds :type Float%20%28single-precision%29))
  (|CallParentFunction DeltaSeconds)
  (switch Utilities|FlowControl|Switch|SwitchonGBaseV2State (Variables|Default|GetCurrent%20State)
    (:NewEnumerator1
      (CallFunction|Battle))))

(fn ConstructionScript
  (|CallParentFunction))

(fn Lockon
  (bind _returnvalue (Transformation|GetActorLocation))
  (bind _as_bp_player_base_v2 (Variables|Default|GetAs%20BP%20Player%20Base%20V2))
  (bind _returnvalue_2 (Transformation|GetActorLocation _as_bp_player_base_v2))
  (bind _returnvalue_3 (Math|Rotator|FindLookatRotation _returnvalue _returnvalue_2))
  (bind (_roll _pitch _yaw) (Math|Rotator|BreakRotator _returnvalue_3))
  (Transformation|SetWorldRotation (Variables|Character|GetMesh) (Math|Rotator|MakeRotator _roll _pitch (+ _yaw -9e+01)) false false))

(fn Battle
  (Utilities|FlowControl|Sequence
    (:then_0
      (CallFunction|Lockon))
    (:then_1
      (if (not (Variables|Default|GetAttack))
        (CallFunction|SettingPullingDirection)
        (Development|PrintString "Setting Pulling Direction Value!" true true "(R=1.000000,G=0.024480,B=0.000000,A=1.000000)")
        (Variables|Default|SetAttack true)
        (Variables|Default|SetCurrent%20Location (Transformation|GetActorLocation))))))

(fn SettingPullingDirection
  (bind _returnvalue (Math|Random|RandomFloatinRange -1.0 1.0))
  (bind _returnvalue_2 (Math|Random|RandomFloatinRange -1.0 1.0))
  (if (> _returnvalue_2 0.25)
    (Utilities|Array|SetArrayElem (Variables|Default|GetPulling%20Direction) 0 1.0)
    (elif (> _returnvalue_2 -0.25)
      (Utilities|Array|SetArrayElem (Variables|Default|GetPulling%20Direction) 0 0.0)
      (else
        (Utilities|Array|SetArrayElem (Variables|Default|GetPulling%20Direction) 0 -1.0))))
  (if (> _returnvalue 0.25)
    (Utilities|Array|SetArrayElem (Variables|Default|GetPulling%20Direction) 1 1.0)
    (elif (> _returnvalue -0.25)
      (Utilities|Array|SetArrayElem (Variables|Default|GetPulling%20Direction) 1 0.0)
      (else
        (Utilities|Array|SetArrayElem (Variables|Default|GetPulling%20Direction) 1 -1.0))))
  (Utilities|FlowControl|Sequence
    (:then_0
      (if (and (Math|Float|NearlyEqual(Float) (Utilities|Array|Get(acopy) (Variables|Default|GetPulling%20Direction)) 0.0 1e-06) (Math|Float|NearlyEqual(Float) (Utilities|Array|Get(acopy) (Variables|Default|GetPulling%20Direction) 1) 0.0 1e-06))
        (if (Math|Random|RandomBool)
          (Utilities|Array|SetArrayElem (Variables|Default|GetPulling%20Direction) 0 1.0)
          (else
            (Utilities|Array|SetArrayElem (Variables|Default|GetPulling%20Direction) 1 1.0)))))
    (:then_1
      (if (and (Math|Float|NearlyEqual(Float) (Utilities|Array|Get(acopy) (Variables|Default|GetPulling%20Direction)) 1.0 1e-06) (Math|Float|NearlyEqual(Float) (Utilities|Array|Get(acopy) (Variables|Default|GetPulling%20Direction) 1) 1.0 1e-06))
        (if (Math|Random|RandomBool)
          (Utilities|Array|SetArrayElem (Variables|Default|GetPulling%20Direction) 0 1.0)
          (else
            (Utilities|Array|SetArrayElem (Variables|Default|GetPulling%20Direction) 1 1.0)))))
    (:then_2
      (if (and (Math|Float|NearlyEqual(Float) (Utilities|Array|Get(acopy) (Variables|Default|GetPulling%20Direction)) -1.0 1e-06) (Math|Float|NearlyEqual(Float) (Utilities|Array|Get(acopy) (Variables|Default|GetPulling%20Direction) 1) -1.0 1e-06))
        (if (Math|Random|RandomBool)
          (Utilities|Array|SetArrayElem (Variables|Default|GetPulling%20Direction) 0 1.0)
          (else
            (Utilities|Array|SetArrayElem (Variables|Default|GetPulling%20Direction) 1 1.0)))))
    (:then_3
      (if (and (Math|Float|NearlyEqual(Float) (Utilities|Array|Get(acopy) (Variables|Default|GetPulling%20Direction)) 1.0 1e-06) (Math|Float|NearlyEqual(Float) (Utilities|Array|Get(acopy) (Variables|Default|GetPulling%20Direction) 1) -1.0 1e-06))
        (if (Math|Random|RandomBool)
          (Utilities|Array|SetArrayElem (Variables|Default|GetPulling%20Direction) 0 1.0)
          (else
            (Utilities|Array|SetArrayElem (Variables|Default|GetPulling%20Direction) 1 1.0)))))
    (:then_4
      (if (and (Math|Float|NearlyEqual(Float) (Utilities|Array|Get(acopy) (Variables|Default|GetPulling%20Direction)) -1.0 1e-06) (Math|Float|NearlyEqual(Float) (Utilities|Array|Get(acopy) (Variables|Default|GetPulling%20Direction) 1) 1.0 1e-06))
        (if (Math|Random|RandomBool)
          (Utilities|Array|SetArrayElem (Variables|Default|GetPulling%20Direction) 0 1.0)
          (else
            (Utilities|Array|SetArrayElem (Variables|Default|GetPulling%20Direction) 1 1.0)))))))